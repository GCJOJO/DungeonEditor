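; BP_SaveManager saves and loads player-editable dungeons made of SpawnablesParent actors.
; Saving gathers strings from Saveable actors into a DungeonSaveData slot with the highest actor MinVersion, refusing overwrites unless forced, plus editor-only debug JSON.
; Loading destroys existing spawnables, respawns each from JSON class, transform and ID, then initializes them in a second pass.
; Old MapSaveParent saves are only flagged, and successful loads update the editor HUD's save name.
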(event `self.ReceiveBeginPlay`
  (`/Game/BPs/DungeonEditorFunctions.WriteToLog` (`KismetStringLibrary.Concat_StrStr` (`KismetSystemLibrary.GetDisplayName` self) " initialized !")))

(fn `GetMinSaveVer`
  (returns (NewerVersion :type String))
  (bind _outactors (`GameplayStatics.GetAllActorsOfClass` "/Game/BPs/Spawnalbes/SpawnablesParent.SpawnablesParent_C"))
  (for _array_element _outactors
    (bind _minversion (`/Game/BPs/Spawnalbes/SpawnablesParent.MinVersion` _array_element))
    (bind (_lefts _rights) (`KismetStringLibrary.Split` _minversion "."))
    (bind (_lefts_2 _rights_2) (`KismetStringLibrary.Split` _rights "."))
    (bind _returnvalue (`KismetStringLibrary.Conv_StringToDouble` (`KismetStringLibrary.Concat_StrStr` _lefts "." _lefts_2 _rights_2)))
    (if (< (`self.NewerVersionFloat`) _returnvalue)
      (set `self.NewerVersionFloat` _returnvalue)
      (set `self.NewerVersionString` _minversion)))
  (return (`self.NewerVersionString`)))

(fn `LoadDungeon`
  (params (SaveName :type String))
  (returns (SaveExists :type Boolean) (bIsOldFormat :type Boolean) (MinSaveVer :type String))
  (locals (CurrentJSONObject :type "BlueprintJsonObject Structure") (CurrentClass :type "/Game/BPs/Spawnalbes/SpawnablesParent Class Reference") (ActorsToInit :type "Map of /Game/BPs/Spawnalbes/SpawnablesParent Object Reference to BlueprintJsonObject Structure"))
  (bind _actorstoinit (`local.ActorsToInit`))
  (bind _returnvalue (`BlueprintJsonLibrary.Conv_JsonValueToString` (`BlueprintJsonLibrary.Conv_JsonObjectToJsonValue` (`local.CurrentJSONObject`) "transform")))
  (bind _returnvalue_2 (`GameplayStatics.DoesSaveGameExist` SaveName))
  (if _returnvalue_2
    (bind _outactors (`GameplayStatics.GetAllActorsOfClass` "/Game/BPs/Spawnalbes/SpawnablesParent.SpawnablesParent_C"))
    (for _array_element _outactors
      (`self.K2_DestroyActor` _array_element))
    (bind _returnvalue_3 (`GameplayStatics.LoadGameFromSlot` (`local.SaveName`)))
    (bind _asdungeon_save_data (cast `/Game/BPs/SaveGames/DungeonSaveData` _returnvalue_3)
      (:`then`
        (`BlueprintMapLibrary.Map_Clear` (`local.ActorsToInit`))
        (bind ((`SaveName` _savename) (`SaveMinVersion` _saveminversion) (`ActorsSaves` _actorssaves)) (break `SaveData` (`/Game/BPs/SaveGames/DungeonSaveData.SaveData` _asdungeon_save_data)))
        (for _array_element_2 _actorssaves
          (bind _output_get (set `local.CurrentJSONObject` (`BlueprintJsonLibrary.Conv_StringToJsonObject` _array_element_2)))
          (bind _asspawnables_parent (castclass `/Game/BPs/Spawnalbes/SpawnablesParent` (`|ConvertAsset` (`KismetSystemLibrary.Conv_SoftClassPathToSoftClassRef` (`KismetSystemLibrary.MakeSoftClassPath` (`BlueprintJsonLibrary.Conv_JsonValueToString` (`BlueprintJsonLibrary.Conv_JsonObjectToJsonValue` _output_get "class")))))))
          (`/Game/BPs/DungeonEditorFunctions.WriteToLog` (`KismetStringLibrary.Concat_StrStr` "Spawning a " (`KismetSystemLibrary.GetClassDisplayName` _asspawnables_parent) " with id " (`KismetStringLibrary.Conv_IntToString` (`BlueprintJsonLibrary.Conv_JsonValueToInteger` (`BlueprintJsonLibrary.Conv_JsonObjectToJsonValue` (`local.CurrentJSONObject`) "actor_id")))))
          (bind _returnvalue_4 (`|SpawnActorFromClass` _asspawnables_parent (`KismetMathLibrary.MakeTransform` (`KismetMathLibrary.MakeVector` (`KismetStringLibrary.Conv_StringToDouble` _returnvalue) (`KismetStringLibrary.Conv_StringToDouble` _returnvalue) (`KismetStringLibrary.Conv_StringToDouble` _returnvalue)) (`KismetMathLibrary.MakeRotator` (`KismetStringLibrary.Conv_StringToDouble` _returnvalue) (`KismetStringLibrary.Conv_StringToDouble` _returnvalue) (`KismetStringLibrary.Conv_StringToDouble` _returnvalue)) (`KismetMathLibrary.MakeVector` (`KismetStringLibrary.Conv_StringToDouble` _returnvalue) (`KismetStringLibrary.Conv_StringToDouble` _returnvalue) (`KismetStringLibrary.Conv_StringToDouble` _returnvalue))) "Undefined" "OverrideRootScale" null true false (`BlueprintJsonLibrary.Conv_JsonValueToInteger` (`BlueprintJsonLibrary.Conv_JsonObjectToJsonValue` (`local.CurrentJSONObject`) "actor_id")) null))
          (`BlueprintMapLibrary.Map_Add` (`local.ActorsToInit`) _returnvalue_4 (`local.CurrentJSONObject`)))
        (bind _keys (`BlueprintMapLibrary.Map_Keys` _actorstoinit))
        (bind _values (`BlueprintMapLibrary.Map_Values` _actorstoinit))
        (for (_array_element_3 _array_index) _keys
          (message `Saveable.LoadSaveData` _array_element_3 (`BlueprintJsonLibrary.Conv_JsonObjectToString` (`|GetArrayItem` _values _array_index))))
        ;[1 1 1] Not a good way to do it but i need the succes return value
        (bind _asdegame_instance (cast `/Game/GameInstance/DEGameInstance` (`GameplayStatics.GetGameInstance`)))
        (`EditableTextBox.SetText` (`/Game/HUD/EditorMenu.SaveNameBox` (`/Game/GameInstance/DEGameInstance.EditorHUD` _asdegame_instance)) (`KismetTextLibrary.Conv_StringToText` _savename))
        (return true false _saveminversion) ; Need to add a bSuccesful return value
      )
      (:`CastFailed`
        (bind (_asmap_save_parent _bsuccess) (cast `/Game/BPs/SaveGames/MapSaveParent` _returnvalue_3 :!pure true))
        (return _bsuccess _bsuccess (`KismetMathLibrary.SelectString` (`.MinVersion_50_AF07396B4687D0BBB172118982B09C22` (break `/Game/Struct/Saves/Save` (`/Game/BPs/SaveGames/MapSaveParent.S_Save` _asmap_save_parent))) "invalid_version" _bsuccess))))
    (else
      (return false false "invalid_version"))))

(fn `SaveDungeon`
  (params (SaveName :type String) (ForceSave :type Boolean))
  (returns (SaveExists :type Boolean))
  (`KismetArrayLibrary.Array_Clear` (`self.Saves`))
  (bind _returnvalue (`GameplayStatics.DoesSaveGameExist` (`local.SaveName`)))
  (if (or (not _returnvalue) (`local.ForceSave`))
    (bind _outactors (`GameplayStatics.GetAllActorsWithInterface` "/Script/DungeonEditor.Saveable"))
    (for _array_element _outactors
      (bind _returnvalue_2 (message `Saveable.SaveSaveData` _array_element))
      (`KismetArrayLibrary.Array_Add` (`self.Saves`) _returnvalue_2))
    (set `self.CurrentSave` (make `SaveData` :`SaveFormatVersion` "2" :`SaveName` (`local.SaveName`) :`SaveMinVersion` (`self.GetMinSaveVer`) :`ActorsSaves` (`self.Saves`)))
    (bind _returnvalue_3 (`GameplayStatics.CreateSaveGameObject` "/Game/BPs/SaveGames/DungeonSaveData.DungeonSaveData_C"))
    (set `/Game/BPs/SaveGames/DungeonSaveData.SaveData` (`self.CurrentSave`) _returnvalue_3)
    (`GameplayStatics.SaveGameToSlot` _returnvalue_3 (`local.SaveName`))
    (if (`DungeonEditorLibrary.IsWithEditor`)
      (`KismetArrayLibrary.Array_Clear` (`self.JsonArray`))
      (for _array_element_2 (`self.Saves`)
        (`KismetArrayLibrary.Array_Add` (`self.JsonArray`) (`BlueprintJsonLibrary.JsonMakeString` _array_element_2)))
      (`/Game/BPs/DungeonEditorFunctions.Write To File (Overwrite)` (`KismetStringLibrary.Concat_StrStr` (`KismetSystemLibrary.GetProjectSavedDirectory`) "SaveGames\\") (`KismetStringLibrary.Concat_StrStr` (`local.SaveName`) ".debug.json") (`BlueprintJsonLibrary.Conv_JsonObjectToPrettyString` (`BlueprintJsonLibrary.JsonMakeField` (`BlueprintJsonLibrary.JsonMakeField` (`BlueprintJsonLibrary.JsonMakeField` (`BlueprintJsonLibrary.JsonMake`) "format_version" (`BlueprintJsonLibrary.JsonMakeString` "2")) "min_save_ver" (`BlueprintJsonLibrary.JsonMakeString` (`self.GetMinSaveVer`))) "actors" (`BlueprintJsonLibrary.JsonMakeArray` (`self.JsonArray`)))))
      (return false)
      (else
        (return false)))
    (else
      (return true))))

(fn `UserConstructionScript`)