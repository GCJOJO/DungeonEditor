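; Spawnable prop for an in-game editor, with click selection that shows X/Y/Z PropEditorArrow gizmo handles and a sphere.
; Clicking SelectionCube toggles selection and binds to every actor's OnClicked, so clicks outside the prop or its children deselect it; clicking one arrow releases the others.
; Play and free-cam modes deselect and hide the billboard, which edit mode shows.
; Construction optionally destroys the arrows and applies collision and forced LOD settings.
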(event `self.ReceiveBeginPlay`
  (bind _xarrow (`self.XArrow`))
  (`parent.ReceiveBeginPlay`)
  (`SceneComponent.SetVisibility` _xarrow (`self.IsSelected`) false)
  (`SceneComponent.SetVisibility` (`self.YArrow`) (`self.IsSelected`) false)
  (`SceneComponent.SetVisibility` (`self.ZArrow`) (`self.IsSelected`) false)
  (`SceneComponent.SetVisibility` (`self.Sphere`) (`self.IsSelected`) false)
  (for _array_element (`|MakeArray` (`ChildActorComponent.ChildActor` (`self.YArrow`)) (`ChildActorComponent.ChildActor` (`self.ZArrow`)) (`ChildActorComponent.ChildActor` _xarrow))
    (bind _asprop_editor_arrow (cast `/Game/BPs/Component/PropEditorArrow` _array_element))
    (set `/Game/BPs/Component/PropEditorArrow.Parent` self _asprop_editor_arrow)
    (add `/Game/BPs/Component/PropEditorArrow.HasBeenClicked` _asprop_editor_arrow (delegate `ArrowClicked`))))

(event `ArrowClicked`
  (params (ArrowClicked :type "/Game/BPs/Component/PropEditorArrow Object Reference"))
  (for _array_element (`|MakeArray` (`ChildActorComponent.ChildActor` (`self.YArrow`)) (`ChildActorComponent.ChildActor` (`self.ZArrow`)) (`ChildActorComponent.ChildActor` (`self.XArrow`)))
    (bind _asprop_editor_arrow (cast `/Game/BPs/Component/PropEditorArrow` _array_element))
    (if (not (== _asprop_editor_arrow ArrowClicked))
      (set `/Game/BPs/Component/PropEditorArrow.IsClicking` false _asprop_editor_arrow)
      (`/Game/BPs/Component/PropEditorArrow.HasBeenReleased` _asprop_editor_arrow))))

(event `self.ReceiveTick`
  (params (DeltaSeconds :type "Float (single-precision)"))
  (`parent.ReceiveTick` DeltaSeconds))

(event `self.SelectionCube.OnClicked`
  (params (TouchedComponent :type "PrimitiveComponent Object Reference") (ButtonPressed :type "Key Structure"))
  (set `self.IsSelected` (not (`self.IsSelected`)))
  (`self.UpdateSelected`)
  (bind _outactors (`GameplayStatics.GetAllActorsOfClass` "/Script/Engine.Actor"))
  (for _array_element _outactors
    (add `self.OnClicked` _array_element (delegate `OtherActorClicked`))))

(event `OtherActorClicked`
  (params (TouchedActor :type "Actor Object Reference") (ButtonPressed :type "Key Structure"))
  (bind _return_value (`self.IsSelfOrChildrenClicked` TouchedActor))
  (if (not (and _return_value (== ButtonPressed "LeftMouseButton")))
    (set `self.IsSelected` false)
    (`self.UpdateSelected`)
    (bind _outactors (`GameplayStatics.GetAllActorsOfClass` "/Script/Engine.Actor"))
    (for _array_element _outactors
      (remove `self.OnClicked` _array_element (delegate `OtherActorClicked`)))))

(fn `EditMode`
  (`parent.EditMode`)
  (`SceneComponent.SetVisibility` (`self.Billboard`) true false))

(fn `FreeCamMode`
  (`parent.FreeCamMode`)
  (`SceneComponent.SetVisibility` (`self.Billboard`) false false)
  (set `self.IsSelected` false)
  (`self.UpdateSelected`))

(fn `IsSelfOrChildrenClicked`
  (params (Actor :type "Actor Object Reference"))
  (returns (`Return Value` :type Boolean))
  (locals (Value :type Boolean))
  (if (== Actor self)
    (set `local.Value` true)
    (else
      (set `local.Value` false)
      (for _array_element (`self.GetAllChildActors` self true)
        (if (== _array_element (`local.Actor`))
          (set `local.Value` true)
          (break)
          (else
            (set `local.Value` false))))))
  (return (`local.Value`)))

(fn `PlayMode`
  (`parent.PlayMode`)
  (`SceneComponent.SetVisibility` (`self.Billboard`) false false)
  (set `self.IsSelected` false)
  (`self.UpdateSelected`))

(fn `UpdateSelected`
  (bind _xarrow (`self.XArrow`))
  (`SceneComponent.SetVisibility` _xarrow (`self.IsSelected`) false)
  (`SceneComponent.SetVisibility` (`self.YArrow`) (`self.IsSelected`) false)
  (`SceneComponent.SetVisibility` (`self.ZArrow`) (`self.IsSelected`) false)
  (`SceneComponent.SetVisibility` (`self.Sphere`) (`self.IsSelected`) false)
  (for _array_element (`|MakeArray` (`ChildActorComponent.ChildActor` (`self.YArrow`)) (`ChildActorComponent.ChildActor` (`self.ZArrow`)) (`ChildActorComponent.ChildActor` _xarrow))
    (bind _asprop_editor_arrow (cast `/Game/BPs/Component/PropEditorArrow` _array_element))
    (set `/Game/BPs/Component/PropEditorArrow.IsParentSelected` (`self.IsSelected`) _asprop_editor_arrow)))

(fn `UserConstructionScript`
  (`parent.UserConstructionScript`)
  (`|ExecutionSequence`
    (:`then_0`
      (if (not (`self.CreateChildActors`))
        (`self.K2_DestroyActor` (`ChildActorComponent.ChildActor` (`self.XArrow`)))
        (`self.K2_DestroyActor` (`ChildActorComponent.ChildActor` (`self.YArrow`)))
        (`self.K2_DestroyActor` (`ChildActorComponent.ChildActor` (`self.ZArrow`)))))
    (:`then_1`
      (`self.SetActorEnableCollision` self (`self.GenerateCollisions`))
      (if (not (== (`self.ForcedLOD`) 0))
        (`StaticMeshComponent.SetForcedLodModel` (`self.Mesh`) (`self.ForcedLOD`))))))