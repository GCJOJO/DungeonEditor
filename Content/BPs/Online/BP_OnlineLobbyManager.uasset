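; Online lobby manager Blueprint that, so far, only logs its initialization on begin play, with no lobby logic yet.
; Its WriteToLog function prints to screen and writes to a dungeon editor log file under the project's Saved/Logs directory.
; It either overwrites the file or appends by loading and re-saving the whole text, writing nothing if that load fails.
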(event `self.OnBeginPlay`
  (`self.WriteToLog` "[OnlineLobbyManager] : OnlineLobbyManager Initialized !"))

(event `self.Tick`
  (params (DeltaTime :type "Float (single-precision)")))

(event `self.OnDestroy`)

(fn `WriteToLog`
  (params (String :type String) (bOverwrite :type Boolean))
  (bind _returnvalue (`KismetStringLibrary.Concat_StrStr` (`local.String`) " \n"))
  (bind (_text _returnvalue_2) (`DungeonEditorLibrary.LoadFile` (`KismetStringLibrary.Concat_StrStr` (`KismetSystemLibrary.GetProjectSavedDirectory`) "/Logs/") "DungeonEditor.dungeon_editor_log"))
  (`KismetSystemLibrary.PrintString` null String)
  (if bOverwrite
    (`DungeonEditorLibrary.SaveFile` (`KismetStringLibrary.Concat_StrStr` (`KismetSystemLibrary.GetProjectSavedDirectory`) "/Logs/") "DungeonEditor.dungeon_editor_log" _returnvalue)
    (elif _returnvalue_2
      (`DungeonEditorLibrary.SaveFile` (`KismetStringLibrary.Concat_StrStr` (`KismetSystemLibrary.GetProjectSavedDirectory`) "/Logs/") "DungeonEditor.dungeon_editor_log" (`KismetStringLibrary.Concat_StrStr` _text _returnvalue)))))