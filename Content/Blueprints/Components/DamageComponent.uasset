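; Damage component that tracks an owner's health and applies damage with temporary invincibility windows.
; HandleDamage ignores hits while recovering; otherwise it clamps the reduced health, broadcasts OnHealthChange with the source details and reports the hit as accepted.
; Timers end recovery after non-lethal hits and after Reset, which restores full health on BeginPlay with initial invincibility.
; At zero health no timer starts, so further damage stays blocked until a reset.
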(event `self.ReceiveBeginPlay`
  (`self.Reset`))

(event `self.ReceiveTick`
  (params (DeltaSeconds :type "Float (single-precision)")))

(event `OnRecovered`
  (set `self.IsRecovering` false))

(fn `HandleDamage`
  (params (Amount :type "Float (double-precision)") (DamageSource :type "Actor Object Reference") (DamageSourceName :type String))
  (returns (Handled :type Boolean))
  (if (not (`self.IsRecovering`))
    (set `self.HealthPoints` (`KismetMathLibrary.FClamp` (- (`self.HealthPoints`) Amount) 0.0 (`self.MaxHealthPoints`)))
    (`self.OnHealthChange` (`local.Amount`) (`local.DamageSource`) (`local.DamageSourceName`))
    (set `self.IsRecovering` true)
    (if (> (`self.HealthPoints`) 0.0)
      (`KismetSystemLibrary.K2_SetTimerDelegate` (`|CreateDelegate` :!event `OnRecovered`) (`self.RecoverTime`)))
    (return true)
    (else
      (return false))))

(fn `Reset`
  (set `self.IsRecovering` true)
  (set `self.HealthPoints` (`self.MaxHealthPoints`))
  (`KismetSystemLibrary.K2_SetTimerDelegate` (`|CreateDelegate` :!event `OnRecovered`) (`self.InitialInvincibleTime`)))