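; Shop inventory component that keeps a list of priced item stacks, with functions to add, remove, look up and reprice them by item ID.
; HasItem linearly searches Items for the index that AddItem uses to merge into existing stacks and GetItem uses for lookups.
; SetPrice and RemoveItem apply Set By Ref to GetItem's result.
; GetItem falls back to a null item from the GlobalActor cached on BeginPlay.
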(event `self.ReceiveBeginPlay`
  (bind _returnvalue (`GameplayStatics.GetActorOfClass` "/Game/Blueprints/System/GlobalActor.GlobalActor_C"))
  (`/Engine/EditorBlueprintResources/StandardMacros.IsValid` _returnvalue
    (:`Is Valid`
      (set `self.GlobalActor` _returnvalue))))

(fn `AddItem`
  (params (ItemName :type Name) (StackAmount :type Integer) (Price :type Integer))
  (bind (_hasitem _itemindex) (`self.HasItem` ItemName))
  (bind _output (`|GetArrayItem` (`self.Items`) _itemindex))
  (bind (_itemstack _price) (break `/Game/Blueprints/Structs/S_ShopItemStack` _output))
  (if _hasitem
    (`|VariableSetRef` _output (make `/Game/Blueprints/Structs/S_ShopItemStack` (make `/Game/Blueprints/Structs/S_ItemStack` (break `/Game/Blueprints/Structs/S_ItemStack` _itemstack) (+ (`.Amount_6_E08F92874EF2B8CDB319CEA713186811` (break `/Game/Blueprints/Structs/S_ItemStack` _itemstack)) (`local.StackAmount`))) _price))
    (else
      (`KismetArrayLibrary.Array_Add` (`self.Items`) (make `/Game/Blueprints/Structs/S_ShopItemStack` (make `/Game/Blueprints/Structs/S_ItemStack` ItemName StackAmount) Price)))))

(fn `GetItem`
  (params (Name :type Name))
  (returns (ShopItem :type "/Game/Blueprints/Structs/S_ShopItemStack Structure"))
  (bind (_hasitem _itemindex) (`self.HasItem` Name))
  (bind _nullitem_nameid (break `/Game/Blueprints/Structs/S_Item` (`/Game/Blueprints/System/GlobalActor.GetNullItem` (`self.GlobalActor`))))
  (return (select `bool` _hasitem :`false` (make `/Game/Blueprints/Structs/S_ShopItemStack` (make `/Game/Blueprints/Structs/S_ItemStack` _nullitem_nameid)) :`true` (`|GetArrayItem` (`self.Items`) _itemindex))))

(fn `HasItem`
  (params (ItemName :type Name))
  (returns (HasItem :type Boolean) (ItemIndex :type Integer))
  (locals (ReturnValue :type Boolean) (Index :type Integer))
  (for (_array_element _array_index) (`self.Items`)
    (if (== (break `/Game/Blueprints/Structs/S_ItemStack` (`.ItemStack_2_DB7E69214024A6D054A5D19C33B72C6B` (break `/Game/Blueprints/Structs/S_ShopItemStack` _array_element))) (`local.ItemName`))
      (set `local.Index` _array_index)
      (set `local.ReturnValue` true)
      (break)))
  (return (`local.ReturnValue`) (`local.Index`)))

(fn `RemoveItem`
  (params (`Item Name` :type Name) (Amount :type Integer))
  (bind _shopitem (`self.GetItem` `Item Name`))
  (bind (_itemstack _price) (break `/Game/Blueprints/Structs/S_ShopItemStack` _shopitem))
  (bind _returnvalue (- (`.Amount_6_E08F92874EF2B8CDB319CEA713186811` (break `/Game/Blueprints/Structs/S_ItemStack` _itemstack)) (`local.Amount`)))
  (if (`self.HasItem` `Item Name`)
    (`|VariableSetRef` _shopitem (make `/Game/Blueprints/Structs/S_ShopItemStack` (make `/Game/Blueprints/Structs/S_ItemStack` (break `/Game/Blueprints/Structs/S_ItemStack` _itemstack) _returnvalue) _price))
    (if (<= _returnvalue 0)
      (`KismetArrayLibrary.Array_RemoveItem` (`self.Items`) _shopitem))))

(fn `SetPrice`
  (params (Name :type Name) (NewPrice :type Integer))
  (bind _shopitem (`self.GetItem` Name))
  (if (`self.HasItem` Name)
    (`|VariableSetRef` _shopitem (make `/Game/Blueprints/Structs/S_ShopItemStack` (`.ItemStack_2_DB7E69214024A6D054A5D19C33B72C6B` (break `/Game/Blueprints/Structs/S_ShopItemStack` _shopitem)) (`local.NewPrice`)))))