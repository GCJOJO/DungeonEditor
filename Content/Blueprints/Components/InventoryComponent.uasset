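; Inventory component that holds an actor's items as an array of ID and amount stacks, with add, remove, query and clear functions.
; Adding looks up the item definition on a lazily cached GlobalActor, merging into an existing stack only if the item is stackable.
; Removal reduces a stack or deletes it when depleted.
; Add and remove broadcast ItemStackChange, though partial removals report a positive amount and full removals a negative one.
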(event `self.ReceiveBeginPlay`
  (bind _returnvalue (`GameplayStatics.GetActorOfClass` "/Game/Blueprints/System/GlobalActor.GlobalActor_C"))
  (`/Engine/EditorBlueprintResources/StandardMacros.IsValid` _returnvalue
    (:`Is Valid`
      (set `self.GlobalActor` _returnvalue))))

(fn `AddItemStack`
  (params (Name :type Name) (Amount :type Integer :default 1))
  (bind (_index _sucess) (`self.GetItemStackIndex` Name))
  (bind _items (`self.Items`))
  (bind (_itemid _amount) (break `/Game/Blueprints/Structs/S_ItemStack` (`|GetArrayItem` _items _index)))
  (bind _globalactor (`self.GetGlobalActor`)
    (:`___`
      (bind (_item _sucess_2) (`/Game/Blueprints/System/GlobalActor.GetItemFromNameId` _globalactor Name))
      (if (and (`.Stackable_22_AA6845B64893FF6DD72ED88492961B24` (break `/Game/Blueprints/Structs/S_Item` _item)) _sucess_2 _sucess)
        (`KismetArrayLibrary.Array_Set` _items _index (make `/Game/Blueprints/Structs/S_ItemStack` _itemid (+ _amount (`local.Amount`))))
        (else
          (`KismetArrayLibrary.Array_Add` (`self.Items`) (make `/Game/Blueprints/Structs/S_ItemStack` (`local.Name`) (`local.Amount`)))))
      (`self.ItemStackChange` (`local.Name`) (`local.Amount`)))))

(fn `ClearInventory`
  (`KismetArrayLibrary.Array_Clear` (`self.Items`)))

(fn `GetItemStack`
  (params (Name :type Name))
  (returns (Stack :type "/Game/Blueprints/Structs/S_ItemStack Structure") (Sucess :type Boolean))
  (locals (Found :type Boolean))
  (for _array_element (`self.Items`)
    (if (== (`.ItemId_3_82BF14E64735743362218C838B013E4E` (break `/Game/Blueprints/Structs/S_ItemStack` _array_element)) (`local.Name`))
      (set `local.Found` true)
      (break)))
  (return _array_element (`local.Found`)))

(fn `GetItemStackIndex`
  (params (Name :type Name))
  (returns (Index :type Integer) (Sucess :type Boolean))
  (locals (Found :type Boolean))
  (for (_array_element _array_index) (`self.Items`)
    (if (== (`.ItemId_3_82BF14E64735743362218C838B013E4E` (break `/Game/Blueprints/Structs/S_ItemStack` _array_element)) (`local.Name`))
      (set `local.Found` true)
      (break)))
  (return _array_index (`local.Found`)))

(fn `GetStackAmount`
  (params (ItemName :type Name))
  (returns (Amount :type Integer))
  (bind (_stack _sucess) (`self.GetItemStack` ItemName))
  (if _sucess
    (return (`.Amount_6_E08F92874EF2B8CDB319CEA713186811` (break `/Game/Blueprints/Structs/S_ItemStack` _stack)))
    (else
      (return 0))))

(fn `HasItemStack`
  (params (Name :type Name))
  (returns (`Has Item Stack` :type Boolean))
  (locals (Found :type Boolean))
  (for _array_element (`self.Items`)
    (if (== (`.ItemId_3_82BF14E64735743362218C838B013E4E` (break `/Game/Blueprints/Structs/S_ItemStack` _array_element)) (`local.Name`))
      (set `local.Found` true)
      (break)))
  (return (`local.Found`)))

(fn `RemoveItemStack`
  (params (Name :type Name) (Amount :type Integer))
  (locals (RemovedAmount :type Integer))
  (bind _index (`self.GetItemStackIndex` Name))
  (bind _items (`self.Items`))
  (bind _amount (`local.Amount`))
  (bind (_itemid _amount_2) (break `/Game/Blueprints/Structs/S_ItemStack` (`self.GetItemStack` Name)))
  (if (`self.HasItemStack` Name)
    (if (<= _amount_2 _amount)
      (set `local.RemovedAmount` (* _amount_2 -1))
      (`KismetArrayLibrary.Array_Remove` _items _index)
      (else
        (set `local.RemovedAmount` _amount)
        (`KismetArrayLibrary.Array_Set` _items _index (make `/Game/Blueprints/Structs/S_ItemStack` _itemid (- _amount_2 (`local.Amount`))))))
    (`self.ItemStackChange` (`local.Name`) (`local.RemovedAmount`))))