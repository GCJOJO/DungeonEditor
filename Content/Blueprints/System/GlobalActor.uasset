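; GlobalActor is a level-wide manager that switches between editor, editor play-test and play modes.
; SetMode spawns or destroys BP_Player, moves controller possession to or from BP_EditorPawn, and notifies every SpawnableObject; full Play Mode destroys the editor pawn and blocks further switches.
; It also provides lookups for spawned objects by ID and items by name ID.
; It saves and loads its creation time as JSON, tagged as the global actor.
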(event `self.ReceiveBeginPlay`
  (set `self.TimeCreated` (`KismetMathLibrary.UtcNow`)))

(event `SetMode`
  (params (`New Mode` :type "GameModeTypes Enum" :default "Editor"))
  (bind _returnvalue (`GameplayStatics.GetPlayerController` 0))
  (bind _returnvalue_2 (`GameplayStatics.GetPlayerController` 0))
  (if (not (`|EnumEquality` (`self.CurrentMode`) "PlayMode"))
    (bind _output_get (set `self.CurrentMode` `New Mode`))
    (switch `GameModeTypes` _output_get
      (:`Editor`
        (bind _returnvalue_3 (`GameplayStatics.GetActorOfClass` "/Game/Blueprints/System/Editor/BP_EditorPawn.BP_EditorPawn_C"))
        (`/Engine/EditorBlueprintResources/StandardMacros.IsValid` _returnvalue_3
          (:`Is Valid`
            (`Controller.UnPossess` _returnvalue)
            (`Controller.Possess` _returnvalue _returnvalue_3))
          (:`Is Not Valid`
            _))
        (bind _returnvalue_4 (`GameplayStatics.GetActorOfClass` "/Game/Blueprints/Player/BP_Player.BP_Player_C"))
        (`/Engine/EditorBlueprintResources/StandardMacros.IsValid` _returnvalue_4
          (:`Is Valid`
            (`self.K2_DestroyActor` _returnvalue_4))
          (:`Is Not Valid`
            _))
        (bind _outactors (`GameplayStatics.GetAllActorsOfClass` "/Game/Blueprints/Objects/SpawnableObject.SpawnableObject_C"))
        (for _array_element _outactors
          (`/Game/Blueprints/Objects/SpawnableObject.EditMode` _array_element)))
      (:`PlayModeEditor`
        (bind _returnvalue_5 (`|SpawnActorFromClass` "/Game/Blueprints/Player/BP_Player.BP_Player_C" (`KismetMathLibrary.MakeTransform` (0.0 0.0 0.0)) "AlwaysSpawn" "MultiplyWithRoot" null null :!label _label))
        (bind _outactors_2 (`GameplayStatics.GetAllActorsOfClass` "/Game/Blueprints/Objects/SpawnableObject.SpawnableObject_C"))
        (for _array_element_2 _outactors_2
          (`/Game/Blueprints/Objects/SpawnableObject.PlayMode` _array_element_2 _returnvalue_5))
        (`Controller.UnPossess` _returnvalue_2)
        (`Controller.Possess` _returnvalue_2 _returnvalue_5))
      (:`PlayMode`
        (bind _returnvalue_6 (`GameplayStatics.GetActorOfClass` "/Game/Blueprints/System/Editor/BP_EditorPawn.BP_EditorPawn_C"))
        (`/Engine/EditorBlueprintResources/StandardMacros.IsValid` _returnvalue_6
          (:`Is Valid`
            (`Controller.UnPossess` (`GameplayStatics.GetPlayerController` 0))
            (`self.K2_DestroyActor` _returnvalue_6)
            (goto _label))
          (:`Is Not Valid`
            (goto _label)))))))

(fn `GetActorWithId`
  (params (ID :type "Guid Structure"))
  (returns (Actor :type "/Game/Blueprints/Objects/SpawnableObject Object Reference") (WasFound :type Boolean))
  (locals (Found :type Boolean))
  (bind _outactors (`GameplayStatics.GetAllActorsOfClass` "/Game/Blueprints/Objects/SpawnableObject.SpawnableObject_C"))
  (for _array_element _outactors
    (if (== (`/Game/Blueprints/Objects/SpawnableObject.Id` _array_element) (`local.ID`))
      (set `local.Found` true)
      (break)))
  (return _array_element (`local.Found`)))

(fn `GetItemFromNameId`
  (params (NameId :type Name))
  (returns (Item :type "/Game/Blueprints/Structs/S_Item Structure") (Sucess :type Boolean))
  (locals (Found :type Boolean))
  (for _array_element (`self.Items`)
    (if (== (`.NameId_2_CC92716C436374FEF07168ADF0251641` (break `/Game/Blueprints/Structs/S_Item` _array_element)) (`local.NameId`))
      (set `local.Found` true)
      (break)))
  (return _array_element (`local.Found`)))

(fn `LoadData`
  (params (Data :type "JsonObjectWrapper Structure"))
  (returns (SaveData :type "JsonObjectWrapper Structure"))
  (bind _outvalue (`|GetJsonField` Data "create_time"))
  (set `self.TimeCreated` _outvalue)
  (return Data))

(fn `SaveData`
  (params (Data :type "JsonObjectWrapper Structure"))
  (returns (SaveData :type "JsonObjectWrapper Structure"))
  (`|SetJsonField` Data "create_time" (`self.TimeCreated`))
  (`|SetJsonField` Data "is_global_actor" (make `EmptyPayload`))
  (return Data))

(fn `UserConstructionScript`)