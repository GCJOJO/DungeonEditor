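; DungeonLibrary is a Blueprint library of helper functions for mouse picking and item lookup.
; GetMouseWorldPos deprojects player 0's cursor and projects the ray onto the Z=0 world plane by scaling its direction, without a line trace.
; GetItemFromName finds the GlobalActor in the level and forwards a name to its GetItemFromNameId, returning the item and a success flag.
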(fn `GetItemFromName`
  (params (ItemName :type Name))
  (returns (Item :type "/Game/Blueprints/Structs/S_Item Structure") (Sucess :type Boolean))
  (bind _returnvalue (`GameplayStatics.GetActorOfClass` null "/Game/Blueprints/System/GlobalActor.GlobalActor_C"))
  (bind (_item _sucess) (`/Game/Blueprints/System/GlobalActor.GetItemFromNameId` _returnvalue ItemName))
  (return _item _sucess))

(fn `GetMouseWorldPos`
  (params (Context :type "Actor Object Reference"))
  (returns (Position :type "Vector Structure"))
  (bind (_worldlocation _worlddirection) (`PlayerController.DeprojectMousePositionToWorld` (`GameplayStatics.GetPlayerController` Context)))
  (return (+ _worldlocation (* (* _worlddirection (/ (.z _worldlocation) (.z _worlddirection))) -1.0))))