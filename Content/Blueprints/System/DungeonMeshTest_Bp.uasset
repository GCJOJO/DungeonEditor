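; Test Blueprint for a voxel-based dungeon mesh, rebuilt by its construction script.
; UpdateTiles queues an Air fill and then a Wall fill over the same size-based cube from the origin, then applies the voxels in one pass.
; Unconnected leftover nodes hold earlier experiments with ModifyVoxelArea, hard-coded floor and wall boxes, and walls placed at actor positions.
; The event graph does nothing.
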(event `self.ReceiveBeginPlay`)

(fn `UpdateTiles`
  (bind _returnvalue (`self.GetSize`))
  (bind _returnvalue_2 (`self.GetSize`))
  (`self.PushVoxelArea` (make `IntVector` 0) (make `IntVector` _returnvalue _returnvalue _returnvalue) "Air")
  (`self.PushVoxelArea` (make `IntVector` 0) (make `IntVector` _returnvalue_2 _returnvalue_2 _returnvalue_2) "Wall")
  (`self.ApplyVoxels`))

(fn `UserConstructionScript`
  (`self.UpdateTiles`))