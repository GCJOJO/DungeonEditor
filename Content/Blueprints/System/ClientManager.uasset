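; ClientManager is an actor that links a player's inventory to on-screen item popups.
; BindToPlayer stores the player behind an IsValid check and binds an event to its InventoryComponent's item stack change.
; ShowPopupUI handles positive amounts only, looking up the item by name through the GlobalActor and adding an ItemPopupUI widget with item and amount to the viewport.
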(event `BindToPlayer`
  (params (Player :type "/Game/Blueprints/Player/BP_Player Object Reference"))
  (`/Engine/EditorBlueprintResources/StandardMacros.IsValid` (`self.Player`)
    (:`Is Not Valid`
      (set `self.Player` Player)
      (add `/Game/Blueprints/Components/InventoryComponent.ItemStackChange` (`/Game/Blueprints/Player/BP_Player.InventoryComponent` Player) (`|CreateDelegate` :!event `ShowPopupUI`)))))

(event `self.ReceiveBeginPlay`)

(event `self.ReceiveTick`
  (params (DeltaSeconds :type "Float (single-precision)")))

(event `ShowPopupUI`
  (params (Name :type Name) (Amount :type Integer))
  (if (> Amount 0)
    (bind _returnvalue (`GameplayStatics.GetActorOfClass` "/Game/Blueprints/System/GlobalActor.GlobalActor_C"))
    (`/Engine/EditorBlueprintResources/StandardMacros.IsValid` _returnvalue
      (:`Is Valid`
        (bind _item (`/Game/Blueprints/System/GlobalActor.GetItemFromNameId` _returnvalue Name))
        (bind _returnvalue_2 (`|CreateWidget` "/Game/UI/Game/Inventory/ItemPopupUI.ItemPopupUI_C" null _item Amount))
        (set `self.ItemPopup` _returnvalue_2)
        (`UserWidget.AddToViewport` (`self.ItemPopup`) 0)))))

(fn `UserConstructionScript`)