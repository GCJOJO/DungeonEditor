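; Dungeon game instance that handles startup, online login, session invites and shared state.
; Init logs a timestamp, attempts auto-login, then shows the info UI and spawns the client manager; login caches achievements, but the LaunchGame progress write is unwired.
; Lazy getters spawn Save and Client manager actors, and a string argument map records state such as InSession.
; Enhanced Input keybinds save to and load from a JSON file in the Saved directory.
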(event `self.ReceiveInit`
  (bind (_year _month _day _hour _minute _second) (`KismetMathLibrary.BreakDateTime` (`KismetMathLibrary.Now`)))
  (`DungeonLibrary.Log` (`KismetStringLibrary.Concat_StrStr` "[DUNGEON EDITOR LOG] " (`KismetStringLibrary.Conv_IntToString` _day) "/" (`KismetStringLibrary.Conv_IntToString` _month) "/" (`KismetStringLibrary.Conv_IntToString` _year) " " (`KismetStringLibrary.Conv_IntToString` _hour) ":" (`KismetStringLibrary.Conv_IntToString` _minute) ":" (`KismetStringLibrary.Conv_IntToString` _second)) true)
  (`|ExecutionSequence`
    (:`then_0`
      (if (`DungeonLibrary.IsEditor`)
        (`KismetSystemLibrary.ExecuteConsoleCommand` "viewmode unlit" (`GameplayStatics.GetPlayerControllerFromID` 0))))
    (:`then_1`
      (`KismetSystemLibrary.Delay` 0.2)
      (`AutoLoginUserCallbackProxy.AutoLoginUser` 0
        (:`then`
          (`DungeonLibrary.Log` "Trying to Auto Login"))
        (:`OnSuccess`
          (`KismetSystemLibrary.DelayUntilNextTick`)
          (`DungeonLibrary.Log` "Sucessfully Auto Logged In")
          (set `self.LoggedIn` true)
          (`KismetSystemLibrary.DelayUntilNextTick` :!label _label)
          (`self.ShowInfoUI`)
          (`self.GetClientManager`))
        (:`OnFailure`
          (`KismetSystemLibrary.DelayUntilNextTick`)
          (`DungeonLibrary.Log` "Couldn't Auto Login")
          (goto _label))))))

(event `ShowInfoUI`
  (`KismetSystemLibrary.DelayUntilNextTick`)
  (bind _returnvalue (`|CreateWidget` "/Game/UI/System/InfoUI.InfoUI_C" null (`self.GameVersion`)))
  (`UserWidget.AddToViewport` _returnvalue 0)
  (add `/Game/UI/System/InfoUI.HasBeenDestroyed` _returnvalue (`|CreateDelegate` :!event `ShowInfoUI`)))

(event `self.OnPlayerLoginStatusChanged`
  (params (PlayerNum :type Integer) (PreviousStatus :type "EBPLoginStatus Enum" :default "NotLoggedIn") (NewStatus :type "EBPLoginStatus Enum" :default "NotLoggedIn") (NewPlayerUniqueNetID :type "BPUniqueNetId Structure"))
  (bind _returnvalue (`GameplayStatics.GetPlayerControllerFromID` 0))
  (if (`|EnumEquality` NewStatus "LoggedIn")
    (`AchievementQueryCallbackProxy.CacheAchievements` _returnvalue
      (:`OnSuccess`
        (`DungeonLibrary.Log` "Cached Achievements" false 10.0))
      (:`OnFailure`
        (`DungeonLibrary.Log` "Couldn't Cache Achievements" false 10.0)))
    (`AchievementQueryCallbackProxy.CacheAchievementDescriptions` _returnvalue
      (:`OnSuccess`
        (`DungeonLibrary.Log` "Cached Achievement Descriptions" false 10.0))
      (:`OnFailure`
        (`DungeonLibrary.Log` "Couldn't Cache Achievement Descriptions" false 10.0)))
    (bind (_bfoundid _progress) (`AchievementBlueprintLibrary.GetCachedAchievementProgress` (`GameplayStatics.GetPlayerControllerFromID` 0) "LaunchGame"))
    (if (< _progress 100.0)
      (`KismetSystemLibrary.Delay` 10.0))))

(event `self.OnSessionInviteAccepted`
  (params (LocalPlayerNum :type Integer) (PersonInvited :type "BPUniqueNetId Structure") (SessionToJoin :type "BlueprintSessionResult Structure (by ref)"))
  (`JoinSessionCallbackProxy.JoinSession` (`GameplayStatics.GetPlayerControllerFromID` 0) SessionToJoin
    (:`OnSuccess`
      (`self.Set Arguments` "InSession" "true"))
    (:`OnFailure`
      (`self.Set Arguments` "InSession" "false"))))

(fn `Get Argument`
  (params (Name :type String))
  (returns (Value :type String) (Found :type Boolean))
  (bind (_value _returnvalue) (`BlueprintMapLibrary.Map_Find` (`self.Arguments`) Name))
  (return _value _returnvalue))

(fn `Get Arguments`
  (returns (Arguments :type "Map of String to String"))
  (return (`self.Arguments`)))

(fn `GetClientManager`
  (returns (ClientManager :type "/Game/Blueprints/System/ClientManager Object Reference"))
  (bind _clientmanagerclass (`self.ClientManagerClass`))
  (`/Engine/EditorBlueprintResources/StandardMacros.IsValid` (`self.ClientManager`)
    (:`Is Valid`
      _)
    (:`Is Not Valid`
      (if (not (`KismetSystemLibrary.IsValidClass` _clientmanagerclass))
        (set `self.ClientManagerClass` "/Game/Blueprints/System/ClientManager.ClientManager_C"))
      (bind _returnvalue (`|SpawnActorFromClass` _clientmanagerclass (`KismetMathLibrary.MakeTransform` (0.0 0.0 0.0)) "Undefined" "SelectDefaultAtRuntime" null null))
      (set `self.ClientManager` _returnvalue)))
  (return (`self.ClientManager`)))

(fn `GetSaveManager`
  (returns (SaveManager :type "/Game/Blueprints/System/SaveManager Object Reference"))
  (bind _savemanagerclass (`self.SaveManagerClass`))
  (`/Engine/EditorBlueprintResources/StandardMacros.IsValid` (`self.SaveManager`)
    (:`Is Valid`
      _)
    (:`Is Not Valid`
      (if (not (`KismetSystemLibrary.IsValidClass` _savemanagerclass))
        (set `self.SaveManagerClass` "/Game/Blueprints/System/SaveManager.SaveManager_C"))
      (bind _returnvalue (`|SpawnActorFromClass` _savemanagerclass (`KismetMathLibrary.MakeTransform` (0.0 0.0 0.0)) "Undefined" "SelectDefaultAtRuntime" null null))
      (set `self.SaveManager` _returnvalue)))
  (return (`self.SaveManager`)))

(fn `LoadKeybinds`
  (locals (Keybinds :type "Map of Name to Key Structure"))
  (bind _returnvalue (`EnhancedInputSubsystemInterface.GetUserSettings` (pcsubsystem `EnhancedInputLocalPlayerSubsystem` (`GameplayStatics.GetPlayerControllerFromID` 0))))
  (`/Engine/EditorBlueprintResources/StandardMacros.IsValid` (`GameplayStatics.GetPlayerControllerFromID` 0)
    (:`Is Valid`
      (bind _outjsonobject (`JsonBlueprintFunctionLibrary.FromFile` (make `FilePath` (`KismetStringLibrary.Concat_StrStr` (`KismetSystemLibrary.GetProjectSavedDirectory`) ".keybinds"))))
      (bind _outvalue (`|GetJsonField` _outjsonobject "keybinds"))
      (bind _output_get (set `local.Keybinds` _outvalue))
      (bind _keys (`BlueprintMapLibrary.Map_Keys` _output_get))
      (bind _values (`BlueprintMapLibrary.Map_Values` _output_get))
      (for (_array_element _array_index) _keys
        (bind _failurereason (`EnhancedInputUserSettings.MapPlayerKey` _returnvalue (make `MapPlayerKeyArgs` _array_element "First" (`|GetArrayItem` _values _array_index) "None" (`EnhancedInputUserSettings.GetActiveKeyProfileId` _returnvalue))))
        (for _array_element_2 (`BlueprintGameplayTagLibrary.BreakGameplayTagContainer` _failurereason)
          (`KismetSystemLibrary.PrintString` (`BlueprintGameplayTagLibrary.GetDebugStringFromGameplayTag` _array_element_2)))))))

(fn `Remove Argument`
  (params (Value :type String))
  (`BlueprintMapLibrary.Map_Remove` (`self.Arguments`) Value))

(fn `SaveKeybinds`
  (locals (Keybinds :type "Map of Name to Key Structure"))
  (bind _jsonobjectwrapper (make `JsonObjectWrapper`))
  (for _array_element (`EnhancedInputSubsystemInterface.GetAllPlayerMappableActionKeyMappings` (pcsubsystem `EnhancedInputLocalPlayerSubsystem` (`GameplayStatics.GetPlayerController` 0)))
    (if (`EnhancedInputLibrary.IsActionKeyMappingPlayerMappable` _array_element)
      (`BlueprintMapLibrary.Map_Add` (`local.Keybinds`) (`EnhancedInputLibrary.GetMappingName` _array_element) (`.Key` (break `EnhancedActionKeyMapping` _array_element)))))
  (`|SetJsonField` _jsonobjectwrapper "keybinds" (`local.Keybinds`))
  (`JsonBlueprintFunctionLibrary.ToFile` _jsonobjectwrapper (make `FilePath` (`KismetStringLibrary.Concat_StrStr` (`KismetSystemLibrary.GetProjectSavedDirectory`) ".keybinds"))))

(fn `Set Arguments`
  (params (Name :type String) (Value :type String))
  (`BlueprintMapLibrary.Map_Add` (`self.Arguments`) Name Value))