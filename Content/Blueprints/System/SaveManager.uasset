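; SaveManager saves and loads dungeons as DungeonSave slot objects holding JSON data.
; Saving gathers JSON from non-child Saveable actors, records the highest SpawnableObject minimum version, and also writes a .json file.
; Loading destroys SpawnableObjects, then, if the game version compares strictly greater, respawns actors by class, skipping duplicate IDs, routes global data to GlobalActor, and finishes with a CompleteLoad pass.
; Version checks OR each component independently, rather than comparing hierarchically.
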(event `LoadActor`
  (params (Class :type "/Game/Blueprints/Objects/SpawnableObject Class Reference") (Transforms :type "Transform Structure") (Data :type "JsonObjectWrapper Structure")))

(fn `CompareVersions`
  (params (A :type String :default "0.0.0") (B :type String :default "0.0.0"))
  (returns (IsA_Highest :type Boolean))
  (bind (_lefts _rights) (`KismetStringLibrary.Split` (`local.A`) "."))
  (bind (_lefts_2 _rights_2) (`KismetStringLibrary.Split` (`local.B`) "."))
  (bind (_lefts_3 _rights_3) (`KismetStringLibrary.Split` _rights "."))
  (bind (_lefts_4 _rights_4) (`KismetStringLibrary.Split` _rights_2 "."))
  (return (or (> (`KismetStringLibrary.Conv_StringToInt` _lefts) (`KismetStringLibrary.Conv_StringToInt` _lefts_2)) (> (`KismetStringLibrary.Conv_StringToInt` _lefts_3) (`KismetStringLibrary.Conv_StringToInt` _lefts_4)) (> (`KismetStringLibrary.Conv_StringToInt` _rights_3) (`KismetStringLibrary.Conv_StringToInt` _rights_4)))))

(fn `GetRequiredMinimumVersion`
  (returns (MinimumVersion :type String))
  (locals (CurrentMinVersion :type String :default "0.0.0"))
  (bind (_lefts _rights) (`KismetStringLibrary.Split` (`local.CurrentMinVersion`) "."))
  (bind (_lefts_2 _rights_2) (`KismetStringLibrary.Split` _rights "."))
  (bind _outactors (`GameplayStatics.GetAllActorsOfClass` "/Game/Blueprints/Objects/SpawnableObject.SpawnableObject_C"))
  (for _array_element _outactors
    (bind _minimumversion (`/Game/Blueprints/Objects/SpawnableObject.MinimumVersion` _array_element))
    (bind (_lefts_3 _rights_3) (`KismetStringLibrary.Split` _minimumversion "."))
    (bind (_lefts_4 _rights_4) (`KismetStringLibrary.Split` _rights_3 "."))
    (if (or (> (`KismetStringLibrary.Conv_StringToInt` _lefts_3) (`KismetStringLibrary.Conv_StringToInt` _lefts)) (> (`KismetStringLibrary.Conv_StringToInt` _lefts_4) (`KismetStringLibrary.Conv_StringToInt` _lefts_2)) (> (`KismetStringLibrary.Conv_StringToInt` _rights_4) (`KismetStringLibrary.Conv_StringToInt` _rights_2)))
      (set `local.CurrentMinVersion` _minimumversion)))
  (return (`local.CurrentMinVersion`)))

(fn `LoadDungeonFromName`
  (params (SaveName :type String))
  (bind _returnvalue (`GameplayStatics.LoadGameFromSlot` (`local.SaveName`)))
  (`/Engine/EditorBlueprintResources/StandardMacros.IsValid` _returnvalue
    (:`Is Valid`
      (bind _asdungeon_save (cast `/Game/Blueprints/System/DungeonSave` _returnvalue))
      (`self.LoadDungeonFromSave` _asdungeon_save))))

(fn `LoadDungeonFromSave`
  (params (Save :type "/Game/Blueprints/System/DungeonSave Object Reference"))
  (locals (SaveGame :type "/Game/Blueprints/System/DungeonSave Object Reference") (SaveData :type "Array of JsonObjectWrapper Structure") (CurrentClass :type "/Game/Blueprints/Objects/SpawnableObject Soft Class Reference") (LoadedIDs :type "Array of Guid Structure"))
  (bind _outactors (`GameplayStatics.GetAllActorsOfClass` "/Game/Blueprints/Objects/SpawnableObject.SpawnableObject_C"))
  (for _array_element _outactors
    (if (not (`self.IsChildActor` _array_element))
      (`self.K2_DestroyActor` _array_element)))
  (`KismetArrayLibrary.Array_Clear` (`local.LoadedIDs`))
  (bind _output_get (set `local.SaveGame` (`local.Save`)))
  (bind _data (`/Game/Blueprints/System/DungeonSave.Data` _output_get))
  (bind _outvalue (`|GetJsonField` _data "min_version"))
  (if (`self.CompareVersions` (`/Game/Blueprints/System/DungeonGameInstance.GameVersion` (cast `/Game/Blueprints/System/DungeonGameInstance` (`GameplayStatics.GetGameInstance`) :!pure true)) _outvalue)
    (bind _outvalue_2 (`|GetJsonField` _data "data"))
    (bind _output_get_2 (set `local.SaveData` _outvalue_2))
    (for _array_element_2 _output_get_2
      (bind _returnvalue (`JsonBlueprintFunctionLibrary.HasField` _array_element_2 "is_global_actor"))
      (if _returnvalue
        (bind _returnvalue_2 (`GameplayStatics.GetActorOfClass` "/Game/Blueprints/System/GlobalActor.GlobalActor_C"))
        (`/Engine/EditorBlueprintResources/StandardMacros.IsValid` _returnvalue_2
          (:`Is Valid`
            (message `/Game/Blueprints/Interfaces/Saveable.LoadData` _returnvalue_2 _array_element_2)))
        (else
          (bind _outvalue_3 (`|GetJsonField` _array_element_2 "id"))
          (if (not (`KismetArrayLibrary.Array_Contains` (`local.LoadedIDs`) _outvalue_3))
            (`KismetArrayLibrary.Array_Add` (`local.LoadedIDs`) _outvalue_3)
            (bind _outvalue_4 (`|GetJsonField` _array_element_2 "class"))
            (bind _output_get_3 (set `local.CurrentClass` _outvalue_4))
            (bind _returnvalue_3 (`|SpawnActorFromClass` (`|ConvertAsset` _output_get_3) (`KismetMathLibrary.MakeTransform` (0.0 0.0 0.0)) "AlwaysSpawn" "SelectDefaultAtRuntime" null null))
            (message `/Game/Blueprints/Interfaces/Saveable.LoadData` _returnvalue_3 _array_element_2)))))
    (bind _outactors_2 (`GameplayStatics.GetAllActorsOfClass` "/Game/Blueprints/Objects/SpawnableObject.SpawnableObject_C"))
    (for _array_element_3 _outactors_2
      (message `/Game/Blueprints/Interfaces/Saveable.CompleteLoad` _array_element_3))))

(fn `SaveDungeon`
  (params (DungeonName :type String))
  (locals (SaveGame :type "/Game/Blueprints/System/DungeonSave Object Reference") (SaveData :type "Array of JsonObjectWrapper Structure"))
  (bind _jsonobjectwrapper (make `JsonObjectWrapper`))
  (bind _savegame (`local.SaveGame`))
  (bind _guid (`/Game/Blueprints/System/DungeonSave.GUID` _savegame))
  (bind _returnvalue (`GameplayStatics.LoadGameFromSlot` DungeonName))
  (`/Engine/EditorBlueprintResources/StandardMacros.IsValid` _returnvalue
    (:`Is Valid`
      (bind _asdungeon_save (cast `/Game/Blueprints/System/DungeonSave` _returnvalue)
        (:`then`
          (set `local.SaveGame` _asdungeon_save))
        (:`CastFailed`
          (bind _returnvalue_2 (`GameplayStatics.CreateSaveGameObject` "/Game/Blueprints/System/DungeonSave.DungeonSave_C" :!label _label))
          (set `local.SaveGame` _returnvalue_2))))
    (:`Is Not Valid`
      (goto _label)))
  (`KismetArrayLibrary.Array_Clear` (`local.SaveData`))
  (set `/Game/Blueprints/System/DungeonSave.Name` (`local.DungeonName`) _savegame)
  (set `/Game/Blueprints/System/DungeonSave.GUID` (select `bool` (`KismetGuidLibrary.IsValid_Guid` _guid) :`false` (`KismetGuidLibrary.NewGuid`) :`true` _guid) _savegame)
  (bind _outactors (`GameplayStatics.GetAllActorsWithInterface` "/Game/Blueprints/Interfaces/Saveable.Saveable_C"))
  (for _array_element _outactors
    (if (not (`self.IsChildActor` _array_element))
      (bind _savedata (message `/Game/Blueprints/Interfaces/Saveable.SaveData` _array_element (make `JsonObjectWrapper`)))
      (`KismetArrayLibrary.Array_Add` (`local.SaveData`) _savedata)))
  (`|SetJsonField` _jsonobjectwrapper "data" (`local.SaveData`))
  (`|SetJsonField` _jsonobjectwrapper "min_version" (`self.GetRequiredMinimumVersion`))
  (bind _output_get (set `/Game/Blueprints/System/DungeonSave.Data` _jsonobjectwrapper _savegame))
  (`JsonBlueprintFunctionLibrary.ToFile` _output_get (make `FilePath` (`KismetStringLibrary.Concat_StrStr` (`KismetSystemLibrary.GetProjectSavedDirectory`) "SaveGames\\" (`local.DungeonName`) ".json")))
  (`GameplayStatics.SaveGameToSlot` _savegame (`local.DungeonName`)))

(fn `UserConstructionScript`)