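; Voxel dungeon mesh that builds floor and walls from the Tile actors placed in the level.
; The construction script calls UpdateTiles, which queues Air over the whole volume and a Floor layer at voxel Y=0.
; Each Tile's location, relative to this actor with a fixed XY offset, becomes a Wall block.
; All queued edits are committed in one ApplyVoxels call, with no active runtime logic.
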(event `self.ReceiveBeginPlay`)

(fn `UpdateTiles`
  (bind _returnvalue (`self.GetSize`))
  (bind _returnvalue_2 (`self.GetSize`))
  (`self.PushVoxelArea` (make `IntVector` 0) (make `IntVector` _returnvalue _returnvalue _returnvalue) "Air")
  (`self.PushVoxelArea` (make `IntVector` 0) (make `IntVector` _returnvalue_2 0 _returnvalue_2) "Floor")
  (bind _outactors (`GameplayStatics.GetAllActorsOfClass` "/Game/Blueprints/Objects/Solid/Tile.Tile_C"))
  (for _array_element _outactors
    (bind _returnvalue_3 (`VoxelFunctionLibrary.WorldToBlockPosition` (- (`self.K2_GetActorLocation` _array_element) (`self.K2_GetActorLocation`) (100.0 100.0 0.0))))
    (`self.PushVoxelArea` _returnvalue_3 _returnvalue_3 "Wall"))
  (`self.ApplyVoxels`))

(fn `UserConstructionScript`
  (`self.UpdateTiles`))