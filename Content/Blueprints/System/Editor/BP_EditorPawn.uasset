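; Player pawn for a grid-based dungeon editor that places, erases and rotates SpawnableObject actors chosen in the EditorUI widget.
; Tick projects the mouse onto the ground and snaps a tinted preview, checking bounds and overlaps; gamepad look moves it via timeline.
; Input places single items or drag-fills areas shown by a procedural box mesh, with the "None" item erasing.
; It also handles pan, zoom and switching modes through GlobalActor.
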(event `EnhancedInput|/Game/Input/Actions/EditorMode/RotateCounterClockwise`
  (params (ActionValue :type Boolean) (ElapsedSeconds :type "Float (double-precision)") (TriggeredSeconds :type "Float (double-precision)") (InputAction :type "InputAction Object Reference" :default "/Game/Input/Actions/EditorMode/RotateCounterClockwise.RotateCounterClockwise"))
  (:`Triggered`
    (`self.Rotate` true)))

(event `EnhancedInput|/Game/Input/Actions/EditorMode/RotateClockwise`
  (params (ActionValue :type Boolean) (ElapsedSeconds :type "Float (double-precision)") (TriggeredSeconds :type "Float (double-precision)") (InputAction :type "InputAction Object Reference" :default "/Game/Input/Actions/EditorMode/RotateClockwise.RotateClockwise"))
  (:`Triggered`
    (`self.Rotate` false)))

(event `self.ReceiveBeginPlay`
  (bind _previewcube (`self.PreviewCube`))
  (set `PlayerController.bShowMouseCursor` true (`GameplayStatics.GetPlayerController` 0))
  (bind _returnvalue (`|CreateWidget` "/Game/UI/System/Editor/EditorUI.EditorUI_C"))
  (set `self.EditorUI` _returnvalue)
  (add `/Game/UI/System/Editor/EditorUI.SelectItem` (`self.EditorUI`) (`|CreateDelegate` :!event `SelectNewItem`))
  (`UserWidget.AddToViewport` (`self.EditorUI`) 0)
  (bind _returnvalue_2 (`PrimitiveComponent.CreateDynamicMaterialInstance` _previewcube 0 (`PrimitiveComponent.GetMaterial` _previewcube 0) "None"))
  (set `self.PreviewCubeMat` _returnvalue_2)
  (`EnhancedInputSubsystemInterface.AddMappingContext` (pcsubsystem `EnhancedInputLocalPlayerSubsystem` (`GameplayStatics.GetPlayerController` 0)) "/Game/Input/DungeonEditorContext.DungeonEditorContext" 0 (struct)))

(event `Key|AnyKey`
  (params (Key :type "Key Structure"))
  (:`Pressed`
    (set `self.UseGamepad` (`KismetInputLibrary.Key_IsGamepadKey` Key))))

(event `self.ReceiveTick`
  (params (DeltaSeconds :type "Float (single-precision)"))
  (bind _previewactor (`self.PreviewActor`))
  (bind _selectionpreview (`self.SelectionPreview`))
  (bind (_worldlocation _worlddirection) (`PlayerController.DeprojectMousePositionToWorld` (`GameplayStatics.GetPlayerController` 0)))
  (bind _x (.x (`self.CurrentPreviewPosition`)))
  (bind _y (.y (`self.CurrentPreviewPosition`)))
  (bind _returnvalue (* 5000.0 -1.0))
  (bind _returnvalue_2 (+ (`SceneComponent.K2_GetComponentLocation` _previewactor) (0.0 0.0 100.0)))
  (bind _returnvalue_3 (+ _worldlocation (* (* _worlddirection (/ (.z _worldlocation) (.z _worlddirection))) -1.0)))
  (set `SpringArmComponent.TargetArmLength` (* (`self.Zoom`) (`self.TileSize`) (`self.ZoomFactor`) 100.0) (`self.SpringArm`))
  (if (not (`self.UseGamepad`))
    (set `self.MouseWorldPos` _returnvalue_3)
    (bind _output_get (set `self.CurrentPreviewPosition` (`KismetMathLibrary.Vector_SnappedToGrid` _returnvalue_3 (`self.GridSize`))))
    (`SceneComponent.K2_SetWorldLocation` (`self.PreviewLag`) _output_get false false)
    (if (== (`.NameId_2_CC92716C436374FEF07168ADF0251641` (break `/Game/Blueprints/Structs/S_Object` (`self.CurrentObject`))) "Selecting")
      (`MaterialInstanceDynamic.SetScalarParameterValue` (`self.PreviewCubeMat`) "Color" 0.44)
      (else
        (if (or (!= (`self.CurrentPreviewPosition`) (`self.LastPreviewPosition`)) (`self.ForcePreviewRefresh`))
          (set `self.CanPlace` true)
          (if (not (and (> _x _returnvalue) (< _x 5000.0) (< _y 5000.0) (> _y _returnvalue)))
            (set `self.CanPlace` false)
            (else
              (bind _outhits (`KismetSystemLibrary.SphereTraceMulti` _returnvalue_2 _returnvalue_2 10.0 "TraceTypeQuery1" false (`|MakeArray` self (`ChildActorComponent.ChildActor` _previewactor) :!type "Actor Object Reference")))
              (for _array_element _outhits
                (if (`KismetMathLibrary.ClassIsChildOf` (`GameplayStatics.GetObjectClass` (`.HitActor` (`GameplayStatics.BreakHitResult` _array_element))) "/Game/Blueprints/Objects/SpawnableObject.SpawnableObject_C")
                  (set `self.CanPlace` false)))))
          (set `self.LastPreviewPosition` (`self.CurrentPreviewPosition`))
          (`MaterialInstanceDynamic.SetScalarParameterValue` (`self.PreviewCubeMat`) "Color" (`KismetMathLibrary.SelectFloat` 0.0 0.344 (`self.CanPlace`)))
          (set `self.ForcePreviewRefresh` false))
        (if (`self.Selecting`)
          (bind (_vertices _triangles _normals _uvs _tangents) (`KismetProceduralMeshLibrary.GenerateBoxMesh` (+ (/ (- (`self.StartPos`) (`self.MouseWorldPos`)) 2) (/ (`self.GridSize`) 2))))
          (`ProceduralMeshComponent.CreateMeshSection_LinearColor` :`self` _selectionpreview :`Vertices` _vertices :`Triangles` _triangles :`Normals` _normals :`UV0` _uvs :`Tangents` _tangents)
          (`SceneComponent.K2_SetWorldLocation` _selectionpreview (+ (/ (+ (`self.StartPos`) (`self.MouseWorldPos`)) 2) (`KismetMathLibrary.MakeVector` 0.0 0.0 101.0)) false false)
          (`PrimitiveComponent.SetMaterial` _selectionpreview 0 "/Game/Materials/Meshes/Cursor.Cursor")
          (else
            (`ProceduralMeshComponent.ClearAllMeshSections` (`self.SelectionPreview`))))))))

(event `EnhancedInput|/Game/Input/Actions/Move`
  (params (ActionValue :type "Vector2D Structure") (ElapsedSeconds :type "Float (double-precision)") (TriggeredSeconds :type "Float (double-precision)") (InputAction :type "InputAction Object Reference" :default "/Game/Input/Actions/Move.Move"))
  (bind (_x _y) (`KismetMathLibrary.BreakVector2D` ActionValue))
  (bind _returnvalue (`SceneComponent.K2_GetComponentLocation` (`self.PreviewActor`)))
  (bind _returnvalue_2 (`KismetMathLibrary.Vector_SnappedToGrid` _returnvalue (`self.GridSize`)))
  (:`Triggered`
    (`|ExecutionSequence`
      (:`then_0`
        (`self.AddMovementInput` (`self.GetActorForwardVector`) (* _x (`self.TileSize`) (`self.Zoom`))))
      (:`then_1`
        (`self.AddMovementInput` (`self.GetActorRightVector`) (* _y (`self.TileSize`) (`self.Zoom`)))))
    (if (!= _returnvalue_2 _returnvalue) :!label _label
      (`SceneComponent.K2_SetWorldLocation` (`self.PreviewLag`) _returnvalue_2 false false)))
  (:`Completed`
    (goto _label)))

(event `EnhancedInput|/Game/Input/Actions/EditorMode/Zoom`
  (params (ActionValue :type "Float (double-precision)") (ElapsedSeconds :type "Float (double-precision)") (TriggeredSeconds :type "Float (double-precision)") (InputAction :type "InputAction Object Reference" :default "/Game/Input/Actions/EditorMode/Zoom.Zoom"))
  (:`Triggered`
    (set `self.Zoom` (`KismetMathLibrary.FClamp` (+ ActionValue (`self.Zoom`)) 2.0 100.0))))

(event `SelectNewItem`
  (params (Item :type "/Game/Blueprints/Structs/S_Object Structure"))
  (bind ((`Class_8_C74B927A40F5F04CA2C94E8915CE2D34` _class) (`SelectionPlaceable_17_D6F175FC479642C1645E9A8B30CAD4BB` _selectionplaceable)) (break `/Game/Blueprints/Structs/S_Object` Item))
  (set `self.CurrentObject` Item)
  (`ChildActorComponent.SetChildActorClass` (`self.PreviewActor`) _class)
  (set `self.UseSelectionToPlace` _selectionplaceable))

(event `EnhancedInput|/Game/Input/Actions/EditorMode/PlaceStart`
  (params (ActionValue :type Boolean) (ElapsedSeconds :type "Float (double-precision)") (TriggeredSeconds :type "Float (double-precision)") (InputAction :type "InputAction Object Reference" :default "/Game/Input/Actions/EditorMode/PlaceStart.PlaceStart"))
  (bind _previewactor (`self.PreviewActor`))
  (bind _childactorclass (`ChildActorComponent.ChildActorClass` (`self.PreviewActor`)))
  (:`Triggered`
    (set `self.StartPos` (`SceneComponent.K2_GetComponentLocation` (`self.PreviewActor`)))
    (if (`self.UseSelectionToPlace`)
      (set `self.Selecting` true)
      (elif (and (`KismetMathLibrary.ClassIsChildOf` _childactorclass "/Game/Blueprints/Objects/SpawnableObject.SpawnableObject_C") (`KismetSystemLibrary.IsValidClass` _childactorclass) (`self.CanPlace`))
        (`|SpawnActorFromClass` (`ChildActorComponent.ChildActorClass` _previewactor) (`KismetMathLibrary.MakeTransform` (`SceneComponent.K2_GetComponentLocation` _previewactor) (`SceneComponent.K2_GetComponentRotation` _previewactor)) "AlwaysSpawn" "SelectDefaultAtRuntime" null null)
        (set `self.ForcePreviewRefresh` true)))))

(event `EnhancedInput|/Game/Input/Actions/EditorMode/PlaceEnd`
  (params (ActionValue :type Boolean) (ElapsedSeconds :type "Float (double-precision)") (TriggeredSeconds :type "Float (double-precision)") (InputAction :type "InputAction Object Reference" :default "/Game/Input/Actions/EditorMode/PlaceEnd.PlaceEnd"))
  (bind _returnvalue (* 5000.0 -1.0))
  (bind _returnvalue_2 (`KismetMathLibrary.FTrunc` (/ (- (.y (`self.EndPos`)) (.y (`self.StartPos`))) (`self.GridSize`))))
  (bind _returnvalue_3 (`KismetMathLibrary.FTrunc` (/ (- (.x (`self.EndPos`)) (.x (`self.StartPos`))) (`self.GridSize`))))
  (bind _returnvalue_4 (< _returnvalue_2 0))
  (bind _returnvalue_5 (< _returnvalue_3 0))
  (:`Triggered`
    (set `self.EndPos` (`SceneComponent.K2_GetComponentLocation` (`self.PreviewActor`)))
    (if (`self.UseSelectionToPlace`)
      (for _index (range (select `bool` _returnvalue_5 :`true` _returnvalue_3) (+ (select `bool` _returnvalue_5 :`false` _returnvalue_3) 1))
        (for _index_2 (range (select `bool` _returnvalue_4 :`true` _returnvalue_2) (+ (select `bool` _returnvalue_4 :`false` _returnvalue_2) 1))
          (bind _returnvalue_6 (`KismetMathLibrary.Vector_SnappedToGrid` (`KismetMathLibrary.MakeVector` (+ (* _index (`self.GridSize`)) (.x (`self.StartPos`))) (+ (* _index_2 (`self.GridSize`)) (.y (`self.StartPos`))) (.z (`self.StartPos`))) (`self.GridSize`)))
          (bind _returnvalue_7 (+ _returnvalue_6 (0.0 0.0 100.0)))
          (bind _outhits (`KismetSystemLibrary.SphereTraceMultiByProfile` _returnvalue_7 _returnvalue_7 50.0 "None" false (`|MakeArray` (`ChildActorComponent.ChildActor` (`self.PreviewActor`)))))
          (for _array_element _outhits
            (bind (_bblockinghit _binitialoverlap _time _distance _location _impactpoint _normal _impactnormal _physmat _hitactor) (`GameplayStatics.BreakHitResult` _array_element))
            (bind _returnvalue_8 (`KismetMathLibrary.ClassIsChildOf` (`GameplayStatics.GetObjectClass` _hitactor) "/Game/Blueprints/Objects/SpawnableObject.SpawnableObject_C"))
            (if _returnvalue_8
              (if (== (`.NameId_2_CC92716C436374FEF07168ADF0251641` (break `/Game/Blueprints/Structs/S_Object` (`self.CurrentObject`))) "None")
                (`self.K2_DestroyActor` _hitactor)
                (else
                  (break)))))
          (bind _x (.x _returnvalue_6))
          (bind _y (.y _returnvalue_6))
          (if (and (not _returnvalue_8) (and (> _x _returnvalue) (< _x 5000.0) (< _y 5000.0) (> _y _returnvalue)))
            (`|SpawnActorFromClass` (`ChildActorComponent.ChildActorClass` (`self.PreviewActor`)) (`KismetMathLibrary.MakeTransform` _returnvalue_6) "AlwaysSpawn" "SelectDefaultAtRuntime" null null))))
      (set `self.Selecting` false))))

(event `self.ReceiveUnpossessed`
  (params (OldController :type "Controller Object Reference"))
  (`SceneComponent.SetVisibility` (`self.CollisionComponent`) false true))

(event `self.ReceivePossessed`
  (params (NewController :type "Controller Object Reference"))
  (`SceneComponent.SetVisibility` (`self.CollisionComponent`) true true)
  (set `PlayerController.bShowMouseCursor` true (`GameplayStatics.GetPlayerController` 0))
  (`/Engine/EditorBlueprintResources/StandardMacros.IsValid` (`self.EditorUI`)
    (:`Is Valid`
      _)
    (:`Is Not Valid`
      (bind _returnvalue (`|CreateWidget` "/Game/UI/System/Editor/EditorUI.EditorUI_C"))
      (set `self.EditorUI` _returnvalue)
      (add `/Game/UI/System/Editor/EditorUI.SelectItem` (`self.EditorUI`) (`|CreateDelegate` :!event `SelectNewItem`))))
  (if (not (`Widget.IsInViewport` (`self.EditorUI`)))
    (`UserWidget.AddToViewport` (`self.EditorUI`) 0)))

(event `EnhancedInput|/Game/Input/Actions/Look`
  (params (ActionValue :type "Vector2D Structure") (ElapsedSeconds :type "Float (double-precision)") (TriggeredSeconds :type "Float (double-precision)") (InputAction :type "InputAction Object Reference" :default "/Game/Input/Actions/Look.Look"))
  (bind (_x _y) (`KismetMathLibrary.BreakVector2D` ActionValue))
  (bind _returnvalue (+ (`self.MouseWorldPos`) (* (`KismetMathLibrary.MakeVector` 0.0 _x) (`self.GridSize`) (`self.GamepadPreviewCubeSpeed`))))
  (bind _returnvalue_2 (+ (`self.MouseWorldPos`) (* (`KismetMathLibrary.MakeVector` (* _y -1.0)) (`self.GridSize`) (`self.GamepadPreviewCubeSpeed`))))
  (:`Triggered`
    (`|ExecutionSequence`
      (:`then_0`
        (if (`self.UseGamepad`)
          (set `self.LastPreviewPosition` (`self.CurrentPreviewPosition`))
          (set `self.MouseWorldPos` _returnvalue)
          (set `self.CurrentPreviewPosition` (`KismetMathLibrary.Vector_SnappedToGrid` _returnvalue (`self.GridSize`)))
          (bind (_direction _alpha) (`Timeline|SmoothPreviewMove` :!via `PlayFromStart` :!label _label_2)
            (:`Update`
              (`SceneComponent.K2_SetWorldLocation` (`self.PreviewLag`) (`KismetMathLibrary.VLerp` (`self.LastPreviewPosition`) (`self.CurrentPreviewPosition`) _alpha) false false)))))
      (:`then_1`
        (if (`self.UseGamepad`)
          (set `self.LastPreviewPosition` (`self.CurrentPreviewPosition`))
          (set `self.MouseWorldPos` _returnvalue_2)
          (set `self.CurrentPreviewPosition` (`KismetMathLibrary.Vector_SnappedToGrid` _returnvalue_2 (`self.GridSize`)))
          (goto _label_2 :!via `PlayFromStart`))))))

(event `EnhancedInput|/Game/Input/Actions/EditorMode/SwitchMode`
  (params (ActionValue :type Boolean) (ElapsedSeconds :type "Float (double-precision)") (TriggeredSeconds :type "Float (double-precision)") (InputAction :type "InputAction Object Reference" :default "/Game/Input/Actions/EditorMode/SwitchMode.SwitchMode"))
  (:`Triggered`
    (bind _returnvalue (`GameplayStatics.GetActorOfClass` "/Game/Blueprints/System/GlobalActor.GlobalActor_C"))
    (`/Engine/EditorBlueprintResources/StandardMacros.IsValid` _returnvalue
      (:`Is Valid`
        (`/Game/Blueprints/System/GlobalActor.SetMode` _returnvalue "PlayModeEditor")
        (`/Game/Blueprints/System/GlobalActor.SetMode` _returnvalue "PlayModeEditor")))))

(fn `Rotate`
  (params (Clowise :type Boolean))
  (bind _previewactor (`self.PreviewActor`))
  (bind ((`NameId_2_CC92716C436374FEF07168ADF0251641` _nameid)) (break `/Game/Blueprints/Structs/S_Object` (`self.CurrentObject`)))
  (bind _returnvalue (+ (`SceneComponent.K2_GetComponentLocation` (`self.PreviewCube`)) (0.0 0.0 50.0)))
  (bind _returnvalue_2 (+ (.yaw (`SceneComponent.K2_GetComponentRotation` _previewactor)) (`KismetMathLibrary.SelectFloat` 90.0 -90.0 (`local.Clowise`))))
  (if (or (== _nameid "Selecting") (== _nameid "None"))
    (bind _outhit (`KismetSystemLibrary.SphereTraceSingle` _returnvalue _returnvalue 50.0 "TraceTypeQuery1"))
    (bind (_bblockinghit _binitialoverlap _time _distance _location _impactpoint _normal _impactnormal _physmat _hitactor) (`GameplayStatics.BreakHitResult` _outhit))
    (`/Engine/EditorBlueprintResources/StandardMacros.IsValid` _hitactor
      (:`Is Valid`
        (bind _returnvalue_3 (+ (.yaw (`self.K2_GetActorRotation` _hitactor)) (`KismetMathLibrary.SelectFloat` 90.0 -90.0 (`local.Clowise`))))
        (`self.K2_SetActorRotation` _hitactor (`KismetMathLibrary.MakeRotator` (.roll (`self.K2_GetActorRotation` _hitactor)) (.pitch (`self.K2_GetActorRotation` _hitactor)) (select `bool` (> _returnvalue_3 360.0) :`false` _returnvalue_3 :`true` 90.0 :!type "Float (single-precision)")) false)))
    (elif (not (`.SelectionPlaceable_17_D6F175FC479642C1645E9A8B30CAD4BB` (break `/Game/Blueprints/Structs/S_Object` (`self.CurrentObject`))))
      (`SceneComponent.K2_SetWorldRotation` _previewactor (`KismetMathLibrary.MakeRotator` (.roll (`SceneComponent.K2_GetComponentRotation` _previewactor)) (.pitch (`SceneComponent.K2_GetComponentRotation` _previewactor)) (select `bool` (> _returnvalue_2 360.0) :`false` _returnvalue_2 :`true` 90.0 :!type "Float (single-precision)")) false false))))

(fn `UserConstructionScript`)