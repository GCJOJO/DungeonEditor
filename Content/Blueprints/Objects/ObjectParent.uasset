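; ObjectParent is a base actor Blueprint for objects that switch between play and edit modes and can be saved and loaded.
; PlayMode hides and EditMode shows the root component and its children when HideOnPlayMode is set, while Reload is an empty stub.
; SaveData writes transform and class fields into JSON wrapper objects, and LoadData reapplies the transform from the supplied JSON.
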(fn `EditMode`
  (if (`self.HideOnPlayMode`)
    (`SceneComponent.SetVisibility` (`self.DefaultSceneRoot`) true true)))

(fn `LoadData`
  (params (Data :type "JsonObjectWrapper Structure"))
  (returns (SaveData :type "JsonObjectWrapper Structure"))
  (bind _outvalue (`|GetJsonField` Data "transforms"))
  (`self.K2_SetActorTransform` _outvalue)
  (return (`local.Data`)))

(fn `PlayMode`
  (params (Player :type "/Game/Player/BP_Player Object Reference"))
  (if (`self.HideOnPlayMode`)
    (`SceneComponent.SetVisibility` (`self.DefaultSceneRoot`) false true)))

(fn `Reload`)

(fn `SaveData`
  (params (Data :type "JsonObjectWrapper Structure"))
  (returns (SaveData :type "JsonObjectWrapper Structure"))
  (bind _jsonobjectwrapper (make `JsonObjectWrapper`))
  (`|SetJsonField` _jsonobjectwrapper "transforms" (`self.GetTransform`))
  (`|SetJsonField` _jsonobjectwrapper "class" (`|ConvertAsset` (`GameplayStatics.GetObjectClass` self)))
  (return _jsonobjectwrapper))

(fn `UserConstructionScript`)