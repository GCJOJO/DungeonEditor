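; Base-style spawnable object actor with a persistent GUID, play/edit mode visibility and JSON save/load.
; Construction and BeginPlay generate a new Id when it is empty, as does LoadData when the saved id is zero.
; SaveData writes transform, class and id to JSON, and LoadData restores transform and id.
; PlayMode and EditMode toggle root visibility if HideOnPlayMode is set; Reload and ChangeActivationState are empty, and Interact just returns true.
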(event `self.ReceiveBeginPlay`
  (if (== (`self.Id`) (`KismetGuidLibrary.Parse_StringToGuid` "{00000000-0000-0000-0000-000000000000}"))
    (set `self.Id` (`KismetGuidLibrary.NewGuid`))))

(fn `ChangeActivationState`
  (params (Activator :type "/Game/Blueprints/Objects/SpawnableObject Object Reference") (Activated :type Boolean)))

(fn `EditMode`
  (if (`self.HideOnPlayMode`)
    (`SceneComponent.SetVisibility` (`self.DefaultSceneRoot`) true true)))

(fn `Interact`
  (params (Source :type "Actor Object Reference"))
  (returns (Return :type Boolean))
  (return true))

(fn `LoadData`
  (params (Data :type "JsonObjectWrapper Structure"))
  (returns (SaveData :type "JsonObjectWrapper Structure"))
  (bind _outvalue (`|GetJsonField` Data "transforms"))
  (`self.K2_SetActorTransform` _outvalue)
  (bind _outvalue_2 (`|GetJsonField` (`local.Data`) "id"))
  (if (== _outvalue_2 (`KismetGuidLibrary.Parse_StringToGuid` "{00000000-0000-0000-0000-000000000000}"))
    (set `self.Id` (`KismetGuidLibrary.NewGuid`))
    (else
      (set `self.Id` _outvalue_2)))
  (return (`local.Data`)))

(fn `PlayMode`
  (params (Player :type "/Game/Blueprints/Player/BP_Player Object Reference"))
  (if (`self.HideOnPlayMode`)
    (`SceneComponent.SetVisibility` (`self.DefaultSceneRoot`) false true)))

(fn `Reload`)

(fn `SaveData`
  (params (Data :type "JsonObjectWrapper Structure"))
  (returns (SaveData :type "JsonObjectWrapper Structure"))
  (bind _jsonobjectwrapper (make `JsonObjectWrapper`))
  (`|SetJsonField` _jsonobjectwrapper "transforms" (`self.GetTransform`))
  (`|SetJsonField` _jsonobjectwrapper "class" (`|ConvertAsset` (`GameplayStatics.GetObjectClass` self)))
  (`|SetJsonField` _jsonobjectwrapper "id" (`self.Id`))
  (return _jsonobjectwrapper))

(fn `UserConstructionScript`
  (if (== (`self.Id`) (`KismetGuidLibrary.Parse_StringToGuid` "{00000000-0000-0000-0000-000000000000}"))
    (set `self.Id` (`KismetGuidLibrary.NewGuid`))))