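; Player controller for the dungeon game that handles player respawning and caches the DEGameInstance on BeginPlay.
; RequestRespawn unpossesses, spawns a half-scale Player just above the first Spawnpoint_S found and possesses it.
; It then calls CallRespawn on the old character, destroys it and resets every SpawnablesParent actor in the level.
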(event `self.ReceiveBeginPlay`
  (`KismetSystemLibrary.PrintString` "Player Controller Initialized")
  (bind _asdegame_instance (cast `/Game/GameInstance/DEGameInstance` (`GameplayStatics.GetGameInstance`)))
  (set `self.Game Instance` _asdegame_instance))

(event `self.ReceiveTick`
  (params (DeltaSeconds :type "Float (single-precision)")))

(event `RequestRespawn`
  (params (OldPlayerChar :type "/Game/Player/Blueprints/Player Object Reference"))
  (`self.UnPossess`)
  (bind _outactors (`GameplayStatics.GetAllActorsOfClass` "/Game/BPs/Spawnalbes/Functions/Spawnpoint_S.Spawnpoint_S_C"))
  (bind (_returnvalue_location _returnvalue_rotation) (`KismetMathLibrary.BreakTransform` (`self.GetTransform` (`|GetArrayItem` _outactors))))
  (bind _returnvalue (`|SpawnActorFromClass` "/Game/Player/Blueprints/Player.Player_C" (`KismetMathLibrary.MakeTransform` (+ _returnvalue_location (`KismetMathLibrary.MakeVector` 0.0 0.0 100.0)) _returnvalue_rotation (0.5 0.5 0.5)) "AdjustIfPossibleButAlwaysSpawn" "OverrideRootScale" self null))
  (`self.Possess` _returnvalue)
  (`/Game/Player/Blueprints/Player.Respawn` OldPlayerChar)
  (`self.K2_DestroyActor` OldPlayerChar)
  (`KismetSystemLibrary.PrintString` "Repsawned")
  (bind _outactors_2 (`GameplayStatics.GetAllActorsOfClass` "/Game/BPs/Spawnalbes/SpawnablesParent.SpawnablesParent_C"))
  (for _array_element _outactors_2
    (`/Game/BPs/Spawnalbes/SpawnablesParent.ResetActor` _array_element)))

(fn `UserConstructionScript`)